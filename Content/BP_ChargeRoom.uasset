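; BP_ChargeRoom is a trigger volume that streams levels in and out as the player crosses it.
; Box overlap by the player character starts OnLevelLoad on entry and OnLevelUnload on exit.
; Each event steps through its LevelToLoad or LevelToUnload array by re-calling itself with an incrementing index, using non-blocking streaming calls and debug prints.
; The indices never reset, and the inclusive length check steps one past the last element.
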(event `self.Box.OnComponentBeginOverlap`
  (params (OverlappedComponent :type "PrimitiveComponent Object Reference") (OtherActor :type "Actor Object Reference") (OtherComp :type "PrimitiveComponent Object Reference") (OtherBodyIndex :type Integer) (bFromSweep :type Boolean) (SweepResult :type "HitResult Structure (by ref)"))
  ;[1 1 1] Begin Overlap
  (if (== OtherActor (`GameplayStatics.GetPlayerCharacter` 0))
    (`self.OnLevelLoad`)))

(event `self.Box.OnComponentEndOverlap`
  (params (OverlappedComponent :type "PrimitiveComponent Object Reference") (OtherActor :type "Actor Object Reference") (OtherComp :type "PrimitiveComponent Object Reference") (OtherBodyIndex :type Integer))
  ;[1 1 1] End Overlap
  (if (== OtherActor (`GameplayStatics.GetPlayerCharacter` 0))
    (`self.OnLevelUnload`)))

(event `OnLevelLoad`
  (bind _level_to_load (`self.Level to Load`))
  ;[1 1 1] Load Levels
  (`GameplayStatics.LoadStreamLevelBySoftObjectPtr` (`|GetArrayItem` _level_to_load (`self.CurrentLoadLevelIndex`)) true)
  (set `self.CurrentLoadLevelIndex` (+ (`self.CurrentLoadLevelIndex`) 1))
  (if (<= (`self.CurrentLoadLevelIndex`) (`KismetArrayLibrary.Array_Length` _level_to_load))
    (`self.OnLevelLoad`)
    (`KismetSystemLibrary.PrintString` "Done Streaming Level" true true (struct :`R` 0.027313 :`G` 1.0 :`A` 1.0))
    (else
      (`KismetSystemLibrary.PrintString` "Stiil Streaming Level" true true (struct :`R` 1.0 :`B` 0.038797 :`A` 1.0)))))

(event `OnLevelUnload`
  (bind _level_to_unload (`self.Level to Unload`))
  ;[1 1 1] Unload Levels
  (`GameplayStatics.UnloadStreamLevelBySoftObjectPtr` (`|GetArrayItem` _level_to_unload (`self.CurrentUnloadLevelIndex`)))
  (set `self.CurrentUnloadLevelIndex` (+ (`self.CurrentUnloadLevelIndex`) 1))
  (if (<= (`self.CurrentUnloadLevelIndex`) (`KismetArrayLibrary.Array_Length` _level_to_unload))
    (`self.OnLevelUnload`)
    (`KismetSystemLibrary.PrintString` "Done Unstreaming Level" true true (struct :`R` 0.027313 :`G` 1.0 :`A` 1.0))
    (else
      (`KismetSystemLibrary.PrintString` "Stiil Unstreaming Level" true true (struct :`R` 1.0 :`B` 0.038797 :`A` 1.0)))))

(fn `UserConstructionScript`)