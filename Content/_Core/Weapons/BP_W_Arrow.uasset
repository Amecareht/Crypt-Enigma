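; Arrow projectile actor that damages what it hits and then destroys itself.
; Construction script configures ProjectileMovement from its Speed, Gravity and Direction variables.
; On a Box hit, actors implementing BPI_ReturnPlayer take the WeaponPDA damage once, with an impact sound.
; Any other hit plays a ground impact sound instead.
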(event `self.Box.OnComponentHit`
  (params (HitComponent :type "PrimitiveComponent Object Reference") (OtherActor :type "Actor Object Reference") (OtherComp :type "PrimitiveComponent Object Reference") (NormalImpulse :type "Vector Structure") (Hit :type "HitResult Structure (by ref)"))
  (if (`KismetSystemLibrary.DoesImplementInterface` OtherActor "/Game/_Core/Blueprints/BPI/BPI_ReturnPlayer.BPI_ReturnPlayer_C")
    (`/Engine/EditorBlueprintResources/StandardMacros.DoOnce` false
      (:`Completed`
        (`GameplayStatics.ApplyDamage` OtherActor (`/Game/_Core/Weapons/DataAsset/PDA_Weapon.Damage` (`self.WeaponPDA`)))
        (`GameplayStatics.PlaySoundAtLocation` "/Game/_Core/Sound/Skeleton/Weapon/Bow/hit_on_ground/Bow_1__impact_.Bow_1__impact_" (`self.K2_GetActorLocation`) (struct) 1.0 1.0 0.0 null null null null)))
    (else
      (`GameplayStatics.PlaySoundAtLocation` "/Game/_Core/Sound/Skeleton/Weapon/Bow/hit_on_ground/Bow_3__impact_ground_.Bow_3__impact_ground_" (`self.K2_GetActorLocation`) (struct) 1.0 1.0 0.0 null null null null)))
  (`self.K2_DestroyActor`))

(fn `UserConstructionScript`
  (bind _projectilemovement (`self.ProjectileMovement`))
  (`parent.UserConstructionScript`)
  (set `ProjectileMovementComponent.InitialSpeed` (`self.Speed`) (`self.ProjectileMovement`))
  (set `ProjectileMovementComponent.MaxSpeed` (`self.Speed`) _projectilemovement)
  (set `ProjectileMovementComponent.ProjectileGravityScale` (`self.Gravity`) _projectilemovement)
  (set `MovementComponent.Velocity` (* (`self.Direction`) (`self.Speed`)) (`self.ProjectileMovement`)))