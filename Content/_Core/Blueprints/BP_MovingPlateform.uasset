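; Moving platform actor that, when Move_Plateform is called, travels from its current location by the EndLocationInMap offset and then returns.
; A timeline lerps the actor out without sweeping, and after a Duration delay a second timeline plays in reverse to bring it back.
; CanReactivate blocks retriggering; its reset follows a delay fired from the return timeline's Update, so it counts from the return's start rather than its finish.
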(event `Move_Plateform`
  (bind _returnvalue (`self.K2_GetActorLocation`))
  (if (`self.Can Reactivate`)
    (set `self.Can Reactivate` false)
    (set `self.Current Location` _returnvalue)
    (set `self.Last Location` (+ _returnvalue (`self.End Location In Map`)))
    (bind (_direction _move_plateform) (`Timeline|Timeline` :!via `PlayFromStart`)
      (:`Update`
        (`self.K2_SetActorLocation` (`KismetMathLibrary.VLerp` (`self.Current Location`) (`self.Last Location`) _move_plateform)))
      (:`Finished`
        (`KismetSystemLibrary.Delay` (`self.Duration`))
        (bind (_direction_2 _remove_plateform) (`Timeline|Timeline_0` :!via `ReverseFromEnd`)
          (:`Update`
            (`self.K2_SetActorLocation` (`KismetMathLibrary.VLerp` (`self.Current Location`) (`self.Last Location`) _remove_plateform))
            (`KismetSystemLibrary.Delay` (`self.Duration`))
            (set `self.Can Reactivate` true)))))))

(fn `UserConstructionScript`)