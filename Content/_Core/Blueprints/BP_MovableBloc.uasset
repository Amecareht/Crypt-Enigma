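; BP_MovableBloc is a block that the horse (BP_Horse) drags along world X through a cable.
; Player pawn overlap with its box attaches and shows the cable, then starts a fast looping timer that polls the horse's position.
; Beyond the cable's range, dot-product and facing checks gate a timeline that lerps the mesh by the horse's last X velocity.
; Only X movement is implemented, and debug prints remain.
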(event `self.ReceiveBeginPlay`
  (set `CableComponent.CableLength` (`self.BaseRangeOfMotion`) (`self.Cable`)))

(event `self.Box.OnComponentBeginOverlap`
  (params (OverlappedComponent :type "PrimitiveComponent Object Reference") (OtherActor :type "Actor Object Reference") (OtherComp :type "PrimitiveComponent Object Reference") (OtherBodyIndex :type Integer) (bFromSweep :type Boolean) (SweepResult :type "HitResult Structure (by ref)"))
  (`KismetSystemLibrary.PrintString` "Hello")
  (if (== OtherActor (`GameplayStatics.GetPlayerPawn` 0))
    (bind _returnvalue (`GameplayStatics.GetActorOfClass` "/Game/UltimateHorsePack/Blueprints/BP_Horse.BP_Horse_C"))
    (bind _output_get (set `self.HorseBP` _returnvalue))
    (`CableComponent.SetAttachEndTo` (`self.Cable`) _output_get "None" "None")
    (bind _returnvalue_2 (`KismetSystemLibrary.K2_SetTimerDelegate` (delegate `SetEndPos`) 0.01 true))
    (set `self.MovingTimer` _returnvalue_2)
    (`SceneComponent.SetVisibility` (`self.Cable`) true false)))

(event `SetEndPos`
  (bind _returnvalue_x (`KismetMathLibrary.BreakVector` (`self.GetActorForwardVector` (`self.HorseBP`))))
  (bind _returnvalue_x_2 (`KismetMathLibrary.BreakVector` (`SceneComponent.GetComponentVelocity` (`Character.CapsuleComponent` (`self.HorseBP`)))))
  (bind _horsebp (`self.HorseBP`)
    (:`then`
      (if (> (`KismetMathLibrary.Vector_Distance` (`self.K2_GetActorLocation` _horsebp) (`self.K2_GetActorLocation`)) (`self.BaseRangeOfMotion`))
        (if (`self.isXMovable`)
          (bind _dotvalue (`self.DotProduct`))
          (`KismetSystemLibrary.PrintString` (`KismetStringLibrary.Conv_DoubleToString` _dotvalue) true false)
          (if (<= (`KismetMathLibrary.Abs` _dotvalue) (`self.BaseRangeOfMotion`))
            (`KismetSystemLibrary.PrintString` "to close of range" false false (struct :`R` 1.0 :`G` 0.008761 :`A` 1.0))
            (elif (== (`KismetMathLibrary.SignOfFloat` _dotvalue) (`KismetMathLibrary.SignOfFloat` _returnvalue_x))
              ;[1 1 1] Bloc Derrière
              (if (`KismetMathLibrary.NearlyEqual_FloatFloat` _returnvalue_x_2 0.0 10.0)
                (bind (_direction _movelerp) (`Timeline|TestMove` :!via `Stop` :!label _label)
                  (:`Update`
                    (`SceneComponent.K2_SetWorldLocation` (`self.StaticMesh`) (`KismetMathLibrary.VLerp` (stale _output_get_2) (`KismetMathLibrary.MakeVector` (+ (.x (stale _output_get_2)) (stale _output_get)) (.y (stale _output_get_2)) (.z (stale _output_get_2))) _movelerp) false false)))
                (else
                  (bind _output_get (set `self.LastVeloX` _returnvalue_x_2))
                  (bind _output_get_2 (set `self.BaseLocation` (`SceneComponent.K2_GetComponentLocation` (`self.StaticMesh`))))
                  (goto _label :!via `PlayFromStart`)))
              (else
                (goto _label :!via `Stop`)))))))
    (:`else`)))

(fn `DotProduct`
  (returns (DotValue :type "Float (double-precision)"))
  (return (`KismetMathLibrary.Dot_VectorVector` (- (`self.K2_GetActorLocation` (`self.HorseBP`)) (`self.K2_GetActorLocation`)) (`SceneComponent.GetForwardVector` (`self.StaticMesh`)))))

(fn `UserConstructionScript`)