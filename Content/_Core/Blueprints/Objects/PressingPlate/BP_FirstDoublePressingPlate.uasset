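; First pressure plate of a two-plate puzzle, reporting to its linked double moving platforms while a BP_Rider overlaps its box.
; On overlap, a timeline lowers the mesh and calls Plate1On on every platform at each update.
; On exit, it calls Plate1NotOn, then, if the platform's MustRemove is set, waits that platform's delay before a second timeline plays in reverse to raise the mesh.
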(event `self.Box.OnComponentBeginOverlap`
  (params (OverlappedComponent :type "PrimitiveComponent Object Reference") (OtherActor :type "Actor Object Reference") (OtherComp :type "PrimitiveComponent Object Reference") (OtherBodyIndex :type Integer) (bFromSweep :type Boolean) (SweepResult :type "HitResult Structure (by ref)"))
  (bind _returnvalue (`self.K2_GetActorLocation`))
  (cast `/Game/UltimateHorsePack/Blueprints/BP_Rider` OtherActor)
  (bind (_direction _newtrack_0) (`Timeline|Timeline_1`)
    (:`Update`
      (`SceneComponent.K2_SetWorldLocation` (`self.StaticMesh`) (`KismetMathLibrary.VLerp` _returnvalue (+ _returnvalue (`self.Going Down In Z`)) _newtrack_0) false false)
      (for _array_element (`self.BP Double Moving Plateform RR`)
        (`/Game/_Core/Blueprints/Objects/MovingPlateform/BP_DoubleMovingPlateformRR.Plate 1 On` _array_element)))))

(event `self.Box.OnComponentEndOverlap`
  (params (OverlappedComponent :type "PrimitiveComponent Object Reference") (OtherActor :type "Actor Object Reference") (OtherComp :type "PrimitiveComponent Object Reference") (OtherBodyIndex :type Integer))
  (bind _returnvalue (`self.K2_GetActorLocation`))
  (cast `/Game/UltimateHorsePack/Blueprints/BP_Rider` OtherActor)
  (for _array_element (`self.BP Double Moving Plateform RR`)
    (`/Game/_Core/Blueprints/Objects/MovingPlateform/BP_DoubleMovingPlateformRR.Plate 1 Not On` _array_element))
  (if (`/Game/_Core/Blueprints/Objects/MovingPlateform/BP_DoubleMovingPlateformRR.Must Remove` _array_element)
    (`KismetSystemLibrary.Delay` (`/Game/_Core/Blueprints/Objects/MovingPlateform/BP_DoubleMovingPlateformRR.Delay Duration` _array_element))
    (bind (_direction _newtrack_0) (`Timeline|Timeline_2` :!via `ReverseFromEnd`)
      (:`Update`
        (`SceneComponent.K2_SetWorldLocation` (`self.StaticMesh`) (`KismetMathLibrary.VLerp` _returnvalue (+ _returnvalue (`self.Going Down In Z`)) _newtrack_0) false false)))))

(fn `Move_Plateform`)

(fn `UserConstructionScript`)