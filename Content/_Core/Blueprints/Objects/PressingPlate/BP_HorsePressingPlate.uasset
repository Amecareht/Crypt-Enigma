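; Pressure plate that responds to BP_Horse overlapping its box and drives linked BPDoubleMovingPlateform actors.
; On entry, a timeline lowers the mesh by GoingDownInZ and repeatedly calls HorseOnPlaque on each platform during its updates.
; On exit, it calls HorseNotOnPlaque, then raises the mesh after the platform's DelayDuration if MustRemove is set.
; DoOnce gates manage the loop and end sounds for each movement.
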(event `self.Box.OnComponentBeginOverlap`
  (params (OverlappedComponent :type "PrimitiveComponent Object Reference") (OtherActor :type "Actor Object Reference") (OtherComp :type "PrimitiveComponent Object Reference") (OtherBodyIndex :type Integer) (bFromSweep :type Boolean) (SweepResult :type "HitResult Structure (by ref)"))
  (bind _returnvalue (`self.K2_GetActorLocation`))
  (bind _returnvalue_2 (`SceneComponent.K2_GetComponentLocation` (`self.StaticMesh`)))
  (bind _returnvalue_3 (`SceneComponent.K2_GetComponentLocation` (`self.StaticMesh`)))
  (cast `/Game/UltimateHorsePack/Blueprints/BP_Horse` OtherActor)
  (bind (_direction _newtrack_0) (`Timeline|Timeline` :!via `PlayFromStart`)
    (:`Update`
      (`SceneComponent.K2_SetWorldLocation` (`self.StaticMesh`) (`KismetMathLibrary.VLerp` _returnvalue (+ _returnvalue (`self.Going Down In Z`)) _newtrack_0) false false)
      (for _array_element (`self.BP_DoubleMovingPlateform`)
        (`/Game/_Core/Blueprints/Objects/MovingPlateform/BP_DoubleMovingPlateformRH.HorseOnPlaque` _array_element)
        (`/Engine/EditorBlueprintResources/StandardMacros.DoOnce` false :!label _label
          (:`Completed`
            (bind _returnvalue_4 (`GameplayStatics.SpawnSoundAtLocation` (`self.Plate Loop Sound`) _returnvalue_3 (struct) 1.0 1.0 0.0 null null))))))
    (:`Finished`
      (`AudioComponent.Stop` _returnvalue_4)
      (`GameplayStatics.SpawnSoundAtLocation` (`self.PlateEndSound`) _returnvalue_3 (struct) 1.0 1.0 0.0 null null)
      (goto _label_2 :!via `Reset`))))

(event `self.Box.OnComponentEndOverlap`
  (params (OverlappedComponent :type "PrimitiveComponent Object Reference") (OtherActor :type "Actor Object Reference") (OtherComp :type "PrimitiveComponent Object Reference") (OtherBodyIndex :type Integer))
  (bind _returnvalue (`self.K2_GetActorLocation`))
  (bind _returnvalue_2 (`SceneComponent.K2_GetComponentLocation` (`self.StaticMesh`)))
  (cast `/Game/UltimateHorsePack/Blueprints/BP_Horse` OtherActor)
  (for _array_element (`self.BP_DoubleMovingPlateform`)
    (`/Game/_Core/Blueprints/Objects/MovingPlateform/BP_DoubleMovingPlateformRH.HorseNotOnPlaque` _array_element))
  (if (`/Game/_Core/Blueprints/Objects/MovingPlateform/BP_DoubleMovingPlateformRH.Must Remove` _array_element)
    (`KismetSystemLibrary.Delay` (`/Game/_Core/Blueprints/Objects/MovingPlateform/BP_DoubleMovingPlateformRH.Delay Duration` _array_element))
    (bind (_direction _newtrack_0) (`Timeline|Timeline_0` :!via `ReverseFromEnd`)
      (:`Update`
        (`SceneComponent.K2_SetWorldLocation` (`self.StaticMesh`) (`KismetMathLibrary.VLerp` _returnvalue (+ _returnvalue (`self.Going Down In Z`)) _newtrack_0) false false)
        (`/Engine/EditorBlueprintResources/StandardMacros.DoOnce` false :!label _label_2
          (:`Completed`
            (bind _returnvalue_3 (`GameplayStatics.SpawnSoundAtLocation` (`self.Plate Loop Sound`) _returnvalue_2 (struct) 1.0 1.0 0.0 null null))
            (goto _label_3 :!via `Reset`))))
      (:`Finished`
        (`AudioComponent.Stop` _returnvalue_3)
        (`/Engine/EditorBlueprintResources/StandardMacros.DoOnce` false :!label _label_3
          (:`Completed`
            (`GameplayStatics.SpawnSoundAtLocation` (`self.PlateEndSound`) _returnvalue_2 (struct) 1.0 1.0 0.0 null null)
            (goto _label :!via `Reset`)))))))

(fn `UserConstructionScript`)