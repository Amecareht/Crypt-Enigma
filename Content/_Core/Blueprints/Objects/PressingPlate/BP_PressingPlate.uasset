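; Pressure plate that drives a list of linked BP_MovingPlateform actors when a horse or rider steps on or off its box.
; Overlap begin calls MovePlateform on each platform and lowers the mesh by GoingDownInZ through a timeline.
; Overlap end notifies each platform, then reverses a second timeline after a delay, gated by MustRemove on the last looped platform.
; Both motions play a loop sound, then an end sound.
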(event `self.Box.OnComponentBeginOverlap`
  (params (OverlappedComponent :type "PrimitiveComponent Object Reference") (OtherActor :type "Actor Object Reference") (OtherComp :type "PrimitiveComponent Object Reference") (OtherBodyIndex :type Integer) (bFromSweep :type Boolean) (SweepResult :type "HitResult Structure (by ref)"))
  (bind _returnvalue (`self.K2_GetActorLocation`))
  (bind _returnvalue_2 (`SceneComponent.K2_GetComponentLocation` (`self.StaticMesh`)))
  ;[1 1 1] Comment
  (cast `/Game/UltimateHorsePack/Blueprints/BP_Horse` OtherActor
    (:`then`
      _)
    (:`CastFailed`
      (cast `/Game/UltimateHorsePack/Blueprints/BP_Rider` OtherActor)))
  (for _array_element (`self.BP_MovingPlateform`)
    (`/Game/_Core/Blueprints/Objects/MovingPlateform/BP_MovingPlateform.Move Plateform` _array_element false)
    (bind (_direction _newtrack_0) (`Timeline|Timeline`)
      (:`Update`
        (`SceneComponent.K2_SetWorldLocation` (`self.StaticMesh`) (`KismetMathLibrary.VLerp` _returnvalue (+ _returnvalue (`self.Going Down In Z`)) _newtrack_0) false false)
        (`/Engine/EditorBlueprintResources/StandardMacros.DoOnce` false :!label _label
          (:`Completed`
            (bind _returnvalue_3 (`GameplayStatics.SpawnSoundAtLocation` (`self.PlateLoopSound`) _returnvalue_2 (struct) 1.0 1.0 0.0 null null)))))
      (:`Finished`
        (`AudioComponent.Stop` _returnvalue_3)
        (`|ExecutionSequence`
          (:`then_0`
            (`GameplayStatics.SpawnSoundAtLocation` (`self.PlateEndSound`) _returnvalue_2 (struct) 1.0 1.0 0.0 null null))
          (:`then_1`
            (goto _label :!via `Reset`)))))))

(event `self.Box.OnComponentEndOverlap`
  (params (OverlappedComponent :type "PrimitiveComponent Object Reference") (OtherActor :type "Actor Object Reference") (OtherComp :type "PrimitiveComponent Object Reference") (OtherBodyIndex :type Integer))
  (bind _returnvalue (`self.K2_GetActorLocation`))
  (bind _returnvalue_2 (`SceneComponent.K2_GetComponentLocation` (`self.StaticMesh`)))
  ;[1 1 1] Comment
  (cast `/Game/UltimateHorsePack/Blueprints/BP_Horse` OtherActor
    (:`then`
      _)
    (:`CastFailed`
      (cast `/Game/UltimateHorsePack/Blueprints/BP_Rider` OtherActor)))
  (for _array_element (`self.BP_MovingPlateform`)
    (`/Game/_Core/Blueprints/Objects/MovingPlateform/BP_MovingPlateform.Left Pression Plate` _array_element))
  (if (`/Game/_Core/Blueprints/Objects/MovingPlateform/BP_MovingPlateform.Must Remove` _array_element)
    (`KismetSystemLibrary.Delay` (`/Game/_Core/Blueprints/Objects/MovingPlateform/BP_MovingPlateform.Delay Duration` _array_element))
    (bind (_direction _newtrack_0) (`Timeline|Timeline_0` :!via `ReverseFromEnd`)
      (:`Update`
        (`SceneComponent.K2_SetWorldLocation` (`self.StaticMesh`) (`KismetMathLibrary.VLerp` _returnvalue (+ _returnvalue (`self.Going Down In Z`)) _newtrack_0) false false)
        (`/Engine/EditorBlueprintResources/StandardMacros.DoOnce` false :!label _label_2
          (:`Completed`
            (bind _returnvalue_3 (`GameplayStatics.SpawnSoundAtLocation` (`self.PlateLoopSound`) _returnvalue_2 (struct) 1.0 1.0 0.0 null null)))))
      (:`Finished`
        (`AudioComponent.Stop` _returnvalue_3)
        (`|ExecutionSequence`
          (:`then_0`
            (`GameplayStatics.SpawnSoundAtLocation` (`self.PlateEndSound`) _returnvalue_2 (struct) 1.0 1.0 0.0 null null))
          (:`then_1`
            (goto _label_2 :!via `Reset`)))))))

(fn `Move_Plateform`)

(fn `UserConstructionScript`)