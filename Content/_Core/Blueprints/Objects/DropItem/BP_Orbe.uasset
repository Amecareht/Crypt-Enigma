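; BP_Orbe is a health orb drop item that heals the player on touch.
; A timeline ping-pongs through the Forward and Reverse events, bobbing Sphere1 above its spawn point and driving a rotation lerp.
; Overlap of Sphere by player pawn 0 passes a DoOnce, calls Heal on its AC_Health component and destroys the orb.
; An uncollected orb destroys itself after TimeBeforeDespawn.
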(event `self.ReceiveBeginPlay`
  (bind (_baselocation_x _baselocation_y _baselocation_z) (`KismetMathLibrary.BreakVector` (`self.BaseLocation`)))
  (`|ExecutionSequence`
    (:`then_0`
      (set `self.BaseLocation` (`self.K2_GetActorLocation`))
      (bind (_direction _location) (`Timeline|MovingTimeline` :!via `PlayFromStart` :!label _label)
        (:`Update`
          (`SceneComponent.K2_SetWorldLocationAndRotation` (`self.Sphere1`) (`KismetMathLibrary.VLerp` (`KismetMathLibrary.MakeVector` _baselocation_x _baselocation_y _baselocation_z) (`KismetMathLibrary.MakeVector` _baselocation_x _baselocation_y (+ _baselocation_z 50.0)) _location) (`KismetMathLibrary.RLerp` (struct) (struct :`Yaw` 360.0) _location true) false false))
        (:`Finished`
          (switch `ETimelineDirection` _direction
            (:`Forward`
              (`self.Reverse`))
            (:`Backward`
              (`self.Forward`))))))
    (:`then_1`
      (`KismetSystemLibrary.Delay` (`self.TimeBeforeDespawn`))
      (`self.K2_DestroyActor`))))

(event `Forward`
  (goto _label :!via `PlayFromStart`))

(event `Reverse`
  (goto _label :!via `Reverse`))

(event `self.Sphere.OnComponentBeginOverlap`
  (params (OverlappedComponent :type "PrimitiveComponent Object Reference") (OtherActor :type "Actor Object Reference") (OtherComp :type "PrimitiveComponent Object Reference") (OtherBodyIndex :type Integer) (bFromSweep :type Boolean) (SweepResult :type "HitResult Structure (by ref)"))
  (bind _returnvalue (`GameplayStatics.GetPlayerPawn` 0))
  (if (== OtherActor _returnvalue)
    (`/Engine/EditorBlueprintResources/StandardMacros.DoOnce` false
      (:`Completed`
        (`/Game/_Core/Blueprints/AC/AC_Health.Heal` (`self.GetComponentByClass` _returnvalue "/Game/_Core/Blueprints/AC/AC_Health.AC_Health_C") (`self.HealDone`))
        (`self.K2_DestroyActor`)))))

(fn `UserConstructionScript`)