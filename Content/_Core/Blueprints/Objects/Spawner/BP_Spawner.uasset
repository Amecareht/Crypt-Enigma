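; Enemy spawner that creates actors from the SpawningPos map, whose keys are positions relative to the spawner and values are the actors to spawn.
; On BeginPlay it enables spawning if the map has entries and starts if CanStartSpawn is set.
; A custom index loop, advanced by RestartForeach, records spawns in SpawnedEnemy.
; DeleteSpawnedUnit removes entries, though its AC_Health OnDeath binding is immediately followed by an unbind-all.
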(event `self.ReceiveBeginPlay`
  (bind _keys (`BlueprintMapLibrary.Map_Keys` (`self.SpawningPos`)))
  (if (> (`KismetArrayLibrary.Array_Length` _keys) 0)
    (set `self.canSpawn` true)
    (bind _keys_2 (`BlueprintMapLibrary.Map_Keys` (`self.SpawningPos`)))
    (set `self.MaxIndex` (`KismetArrayLibrary.Array_Length` _keys_2))
    (if (`self.CanStartSpawn`)
      (`self.SpawningEnemy`))
    (else
      (set `self.canSpawn` false))))

(event `RestartForeach`
  (bind _spawningpos (`self.SpawningPos`))
  ;[1 1 1] Add 1 to the loop
  (`/Engine/EditorBlueprintResources/StandardMacros.IncrementInt` (`self.CurrentIndex`)
    (:`  `
      ;[0.01347 0.6121 0.344] Foreach custom
      (if (not (== (`self.CurrentIndex`) (`self.MaxIndex`))) :!label _label
        (bind _keys (`BlueprintMapLibrary.Map_Keys` _spawningpos))
        (bind _values (`BlueprintMapLibrary.Map_Values` _spawningpos))
        (`self.SpawningActors` (`|GetArrayItem` _keys (`self.CurrentIndex`)) (`|GetArrayItem` _values (`self.CurrentIndex`)))))))

(event `SpawningEnemy`
  ;[0.01347 0.6121 0.344] Foreach custom
  (if (`self.canSpawn`)
    (set `self.CurrentIndex` 0)
    (goto _label)))

(event `SpawningActors`
  (params (LocationToSPawn :type "Vector Structure") (ActorToSPawn :type "Actor Object Reference"))
  (bind _returnvalue (`self.GetComponentByClass` "/Game/_Core/Blueprints/AC/AC_Health.AC_Health_C"))
  ;[1 0.07248 0.2376] SPawning actor & bind event OnDeath
  (bind _returnvalue_2 (`|SpawnActorFromClass` (`GameplayStatics.GetObjectClass` ActorToSPawn) (`KismetMathLibrary.MakeTransform` (+ LocationToSPawn (`self.K2_GetActorLocation`))) "Undefined" "MultiplyWithRoot" null null))
  (`KismetArrayLibrary.Array_Add` (`self.SpawnedEnemy`) _returnvalue_2)
  (`/Engine/EditorBlueprintResources/StandardMacros.IsValid` _returnvalue
    (:`Is Valid`
      (add `/Game/_Core/Blueprints/AC/AC_Health.OnDeath` _returnvalue (delegate `DeleteSpawnedUnit`))
      (clear `/Game/_Core/Blueprints/AC/AC_Health.OnDeath` _returnvalue)
      (`KismetSystemLibrary.DelayUntilNextTick`))))

(event `DeleteSpawnedUnit`
  (params (RefToSelf :type "Actor Object Reference"))
  ;[1 0.07248 0.2376] SPawning actor & bind event OnDeath
  (`KismetArrayLibrary.Array_RemoveItem` (`self.SpawnedEnemy`) RefToSelf))

(fn `UserConstructionScript`)