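; BP_RiderPressingPlate is a pressure plate that responds only to BP_Rider and drives the double moving platforms.
; Its Box overlap begin and end events cast the other actor to BP_Rider, then find every BP_DoubleMovingPlateform in the level.
; Each platform receives RiderOnPlaque on entry and RiderNotOnPlaque on exit, so the plate affects all of them rather than a linked instance.
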(event `self.Box.OnComponentBeginOverlap`
  (params (OverlappedComponent :type "PrimitiveComponent Object Reference") (OtherActor :type "Actor Object Reference") (OtherComp :type "PrimitiveComponent Object Reference") (OtherBodyIndex :type Integer) (bFromSweep :type Boolean) (SweepResult :type "HitResult Structure (by ref)"))
  (cast `/Game/UltimateHorsePack/Blueprints/BP_Rider` OtherActor)
  (`GameplayStatics.GetAllActorsOfClass` "/Game/_Core/Blueprints/Objects/BP_DoubleMovingPlateform.BP_DoubleMovingPlateform_C")
  (for _array_element (`self.BP_DoubleMovingPlateform`)
    (`/Game/_Core/Blueprints/Objects/BP_DoubleMovingPlateform.RiderOnPlaque` _array_element)))

(event `self.Box.OnComponentEndOverlap`
  (params (OverlappedComponent :type "PrimitiveComponent Object Reference") (OtherActor :type "Actor Object Reference") (OtherComp :type "PrimitiveComponent Object Reference") (OtherBodyIndex :type Integer))
  (cast `/Game/UltimateHorsePack/Blueprints/BP_Rider` OtherActor)
  (`GameplayStatics.GetAllActorsOfClass` "/Game/_Core/Blueprints/Objects/BP_DoubleMovingPlateform.BP_DoubleMovingPlateform_C")
  (for _array_element (`self.BP_DoubleMovingPlateform`)
    (`/Game/_Core/Blueprints/Objects/BP_DoubleMovingPlateform.RiderNotOnPlaque` _array_element)))

(fn `UserConstructionScript`)