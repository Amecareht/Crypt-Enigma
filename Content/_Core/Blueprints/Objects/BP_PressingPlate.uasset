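; BP_PressingPlate is a pressure plate that drives every BP_MovingPlateform in the level when BP_Horse or BP_Rider overlaps its box.
; On overlap, a timeline lerps the plate mesh by GoingDownInZ and calls MovePlateform on all platforms each update.
; On exit, it calls LeftPressionPlate on each platform, then reverses a second timeline after a platform's DelayDuration to restore the mesh.
; The plate's own MovePlateform function is empty.
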(event `self.Box.OnComponentBeginOverlap`
  (params (OverlappedComponent :type "PrimitiveComponent Object Reference") (OtherActor :type "Actor Object Reference") (OtherComp :type "PrimitiveComponent Object Reference") (OtherBodyIndex :type Integer) (bFromSweep :type Boolean) (SweepResult :type "HitResult Structure (by ref)"))
  (bind _returnvalue (`self.K2_GetActorLocation`))
  (`|ExecutionSequence`
    (:`then_0`
      (cast `/Game/UltimateHorsePack/Blueprints/BP_Horse` OtherActor))
    (:`then_1`
      (cast `/Game/UltimateHorsePack/Blueprints/BP_Rider` OtherActor)))
  (`GameplayStatics.GetAllActorsOfClass` "/Game/_Core/Blueprints/Objects/BP_MovingPlateform.BP_MovingPlateform_C")
  (bind (_direction _newtrack_0) (`Timeline|Timeline` :!via `PlayFromStart`)
    (:`Update`
      (`SceneComponent.K2_SetWorldLocation` (`self.StaticMesh`) (`KismetMathLibrary.VLerp` _returnvalue (+ _returnvalue (`self.Going Down In Z`)) _newtrack_0) false false)
      (for _array_element (`self.BP_MovingPlateform`)
        (`/Game/_Core/Blueprints/Objects/BP_MovingPlateform.Move Plateform` _array_element)))))

(event `self.Box.OnComponentEndOverlap`
  (params (OverlappedComponent :type "PrimitiveComponent Object Reference") (OtherActor :type "Actor Object Reference") (OtherComp :type "PrimitiveComponent Object Reference") (OtherBodyIndex :type Integer))
  (bind _returnvalue (`self.K2_GetActorLocation`))
  (`|ExecutionSequence`
    (:`then_0`
      (cast `/Game/UltimateHorsePack/Blueprints/BP_Horse` OtherActor))
    (:`then_1`
      (cast `/Game/UltimateHorsePack/Blueprints/BP_Rider` OtherActor)))
  (`GameplayStatics.GetAllActorsOfClass` "/Game/_Core/Blueprints/Objects/BP_MovingPlateform.BP_MovingPlateform_C")
  (for _array_element (`self.BP_MovingPlateform`)
    (`|ExecutionSequence`
      (:`then_0`
        (`/Game/_Core/Blueprints/Objects/BP_MovingPlateform.Left Pression Plate` _array_element))
      (:`then_1`
        (`KismetSystemLibrary.Delay` (`/Game/_Core/Blueprints/Objects/BP_MovingPlateform.Delay Duration` _array_element))
        (bind (_direction _newtrack_0) (`Timeline|Timeline_0` :!via `ReverseFromEnd`)
          (:`Update`
            (`SceneComponent.K2_SetWorldLocation` (`self.StaticMesh`) (`KismetMathLibrary.VLerp` _returnvalue (+ _returnvalue (`self.Going Down In Z`)) _newtrack_0) false false)))))))

(fn `Move_Plateform`)

(fn `UserConstructionScript`)