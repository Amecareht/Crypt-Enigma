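; Moving platform that travels by an offset when both the rider and horse pressure-plate flags are set.
; Plate events update the flags and trigger the move or return, gated by CanRemove and CanReactivate so trips finish before reversing or restarting.
; Timelines lerp the actor between endpoints, with play rate scaled by speed over distance.
; The return waits a delay before starting and another before re-arming.
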(event `HorseNotOnPlaque`
  (set `self.Horse` false)
  (`self.Re Move Plateform`))

(event `RiderOnPlaque`
  (set `self.Rider` true)
  (`self.Move Plateform`))

(event `HorseOnPlaque`
  (set `self.Horse` true)
  (`self.Move Plateform`))

(event `RiderNotOnPlaque`
  (set `self.Rider` false)
  (`self.Re Move Plateform`))

(event `Move Plateform`
  (bind _returnvalue (`self.K2_GetActorLocation`))
  (if (and (`self.Rider`) (`self.Horse`))
    (set `self.Player And Horse On Pression Plate` true)
    (set `self.Can Remove` false)
    (if (`self.Can Reactivate`)
      (set `self.Can Reactivate` false)
      (set `self.First Location` _returnvalue)
      (set `self.Last Location` (+ _returnvalue (`self.End Location In Map`)))
      (`TimelineComponent.SetPlayRate` (`self.Timeline`) (/ (* (`self.Speed`) 1000.0) (`KismetMathLibrary.Vector_Distance` (`self.K2_GetActorLocation`) (`self.Last Location`))))
      (bind (_direction _move_plateform) (`Timeline|Timeline` :!via `PlayFromStart`)
        (:`Update`
          (`self.K2_SetActorLocation` (`KismetMathLibrary.VLerp` (`self.First Location`) (`self.Last Location`) _move_plateform)))
        (:`Finished`
          (set `self.Can Remove` true)
          (if (`self.Player And Horse On Pression Plate`)
            _
            (elif (`self.Must Remove`)
              (`self.Re Move Plateform`))))))
    (else
      (`self.Re Move Plateform`))))

(event `Left Pression Plate`
  (set `self.Player And Horse On Pression Plate` false)
  (`self.Re Move Plateform`))

(event `Re Move Plateform`
  (if (`self.Can Remove`)
    (`KismetSystemLibrary.Delay` (`self.Delay Duration`))
    (`TimelineComponent.SetPlayRate` (`self.Timeline_0`) (/ (* (`self.Speed`) 1000.0) (`KismetMathLibrary.Vector_Distance` (`self.Last Location`) (`self.First Location`))))
    (bind (_direction _remove_plateform) (`Timeline|Timeline_0` :!via `ReverseFromEnd`)
      (:`Update`
        (`self.K2_SetActorLocation` (`KismetMathLibrary.VLerp` (`self.First Location`) (`self.Last Location`) _remove_plateform)))
      (:`Finished`
        (`KismetSystemLibrary.Delay` (`self.Delay Duration`))
        (set `self.Can Reactivate` true)))))

(fn `UserConstructionScript`)