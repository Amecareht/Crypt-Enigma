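; Moving platform driven by two pressure plates: it travels by an offset once both plates are active.
; Plate events set flags, with a delay on release, and a timeline lerps the actor to the target.
; If MustRemove is set, a second timeline reverses it home after both plates release and the outward move finishes.
; Play rates divide Speed by distance for consistent velocity, while flags and delays gate reactivation.
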(event `Plate 1 On`
  ;[1 1 1] Plate 1 Activation
  (set `self.Plate1` true)
  (`self.Move Plateform`))

(event `Plate2On`
  ;[1 1 1] Plate 2 Activation
  (set `self.Plate2` true)
  (`self.Move Plateform`))

(event `Plate 1 Not On`
  ;[1 1 1] Plate 1 Activation
  (`KismetSystemLibrary.Delay` (`self.Wait Before Deactivate`))
  (set `self.Plate1` false)
  (`self.Re Move Plateform`))

(event `Plate2NotOn`
  ;[1 1 1] Plate 2 Activation
  (`KismetSystemLibrary.Delay` (`self.Wait Before Deactivate`))
  (set `self.Plate2` false)
  (`self.Re Move Plateform`))

(event `Move Plateform`
  (bind _returnvalue (`self.K2_GetActorLocation`))
  ;[1 1 1] First Move Plateform
  (if (and (`self.Plate1`) (`self.Plate2`))
    (set `self.2 Plates On` true)
    (set `self.Can Remove` false)
    (if (`self.Can Reactivate`)
      (set `self.Can Reactivate` false)
      (set `self.First Location` _returnvalue)
      (set `self.Last Location` (+ _returnvalue (`self.End Location In Map`)))
      (`TimelineComponent.SetPlayRate` (`self.Timeline`) (/ (* (`self.Speed`) 1000.0) (`KismetMathLibrary.Vector_Distance` (`self.K2_GetActorLocation`) (`self.Last Location`))))
      (bind (_direction _move_plateform) (`Timeline|Timeline` :!via `PlayFromStart`)
        (:`Update`
          (`self.K2_SetActorLocation` (`KismetMathLibrary.VLerp` (`self.First Location`) (`self.Last Location`) _move_plateform)))
        (:`Finished`
          (set `self.Can Remove` true)
          (if (`self.2 Plates On`)
            _
            (elif (`self.Must Remove`)
              (`self.Re Move Plateform`))))))
    (else
      (`self.Re Move Plateform`))))

(event `Left Pression Plate`
  ;[1 1 1] Preparation for remove
  (set `self.2 Plates On` false)
  (`self.Re Move Plateform`))

(event `Re Move Plateform`
  ;[1 1 1] Remove Plateform
  (if (`self.Must Remove`)
    (if (or (`self.Plate1`) (`self.Plate2`))
      _
      (elif (`self.Can Remove`)
        (`KismetSystemLibrary.Delay` (`self.Delay Duration`))
        (`TimelineComponent.SetPlayRate` (`self.Timeline_0`) (/ (* (`self.Speed`) 1000.0) (`KismetMathLibrary.Vector_Distance` (`self.Last Location`) (`self.First Location`))))
        (bind (_direction _remove_plateform) (`Timeline|Timeline_0` :!via `ReverseFromEnd`)
          (:`Update`
            (`self.K2_SetActorLocation` (`KismetMathLibrary.VLerp` (`self.First Location`) (`self.Last Location`) _remove_plateform)))
          (:`Finished`
            (`KismetSystemLibrary.Delay` (`self.Delay Duration`))
            (set `self.Can Reactivate` true)))))))

(fn `UserConstructionScript`)