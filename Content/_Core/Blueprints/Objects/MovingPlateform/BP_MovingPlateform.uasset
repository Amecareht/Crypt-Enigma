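; Moving platform driven by pressure-plate events, sliding from its placed location to an offset EndLocationInMap and back.
; MovePlateform runs a forward timeline, and the return plays a second one in reverse after a delay, with play rates scaled by Speed over distance.
; Leaving the plate triggers the return once travel has finished; a departure mid-travel returns on arrival only if MustRemove is set.
; CanReactivate blocks retriggering until the return and a final delay finish.
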(event `Move Plateform`
  (bind _returnvalue (`self.K2_GetActorLocation`))
  (set `self.Player On Pression Plate` true)
  (set `self.Can Remove` false)
  (if (`self.Can Reactivate`)
    (set `self.Can Reactivate` false)
    (set `self.First Location` _returnvalue)
    (set `self.Last Location` (+ _returnvalue (`self.End Location In Map`)))
    (`TimelineComponent.SetPlayRate` (`self.Timeline_1`) (/ (* (`self.Speed`) 1000.0) (`KismetMathLibrary.Vector_Distance` (`self.K2_GetActorLocation`) (`self.Last Location`))))
    (bind (_direction _move_plateform) (`Timeline|Timeline_1` :!via `PlayFromStart`)
      (:`Update`
        (`self.K2_SetActorLocation` (`KismetMathLibrary.VLerp` (`self.First Location`) (`self.Last Location`) _move_plateform)))
      (:`Finished`
        (set `self.Can Remove` true)
        (if (`self.Player On Pression Plate`)
          _
          (elif (`self.Must Remove`)
            (`self.Re Move Plateform`)))))))

(event `Left Pression Plate`
  (bind _outactors (`GameplayStatics.GetAllActorsOfClass` "/Game/_Core/Blueprints/Objects/PressingPlate/BP_PressingPlate.BP_PressingPlate_C"))
  (set `self.Player On Pression Plate` false)
  (`self.Re Move Plateform`))

(event `Re Move Plateform`
  (if (`self.Can Remove`)
    (`KismetSystemLibrary.Delay` (`self.Delay Duration`))
    (`TimelineComponent.SetPlayRate` (`self.Timeline_2`) (/ (* (`self.Speed`) 1000.0) (`KismetMathLibrary.Vector_Distance` (`self.Last Location`) (`self.First Location`))))
    (bind (_direction _remove_plateform) (`Timeline|Timeline_2` :!via `ReverseFromEnd`)
      (:`Update`
        (`self.K2_SetActorLocation` (`KismetMathLibrary.VLerp` (`self.First Location`) (`self.Last Location`) _remove_plateform)))
      (:`Finished`
        (`KismetSystemLibrary.Delay` (`self.Delay Duration`))
        (set `self.Can Reactivate` true)))))

(fn `UserConstructionScript`)