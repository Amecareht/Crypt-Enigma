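; Grappling hook component for BP_ThirdPersonCharacter that launches the player toward Grapplable surfaces and swings them on a rope.
; StartTraceGrapple traces from the hand along camera forward, launches with a wheel-input sideways bias, and starts a reload cooldown.
; After a short delay, it spawns Bp_Rope at the impact, constraining the physics-simulated capsule to it.
; Right mouse or a failed trace cancels, restoring falling movement, destroying any rope and keeping partial momentum.
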(event `CE_CancelHookTrace`
  (bind _returnvalue (* (`Actor.GetVelocity` (`self.Owner`)) 0.75))
  (`self.CancelGrappin` :!label _label)
  (set `self.bHasUsedGrap` false)
  (set `self.bGrapplingJump` false)
  (bind _rope (`self.Rope`)
    (:`then`
      (`Actor.K2_DestroyActor` _rope)
      (`KismetSystemLibrary.PrintString` (`KismetStringLibrary.Conv_VectorToString` _returnvalue) true true (struct :`G` 0.66 :`B` 1.0 :`A` 1.0) 20.0)
      (set `MovementComponent.Velocity` _returnvalue (`Character.CharacterMovement` (`self.Owner`))))
    (:`else`)))

(event `Key|RightMouseButton`
  (params (Key :type "Key Structure"))
  (:`Pressed`
    (goto _label)))

(event `self.ReceiveBeginPlay`
  (bind _asbp_third_person_character (cast `/Game/_Core/ThirdPerson/Blueprints/BP_ThirdPersonCharacter` (`self.GetOwner`)))
  (set `self.Owner` _asbp_third_person_character))

(event `StartTraceGrapple`
  (params (`WheelMouse input` :type "Float (double-precision)"))
  (bind _owner (`self.Owner`))
  (bind _capsulecomponent (`Character.CapsuleComponent` (`self.Owner`)))
  (bind _returnvalue (`SceneComponent.K2_GetComponentLocation` (`/Game/_Core/ThirdPerson/Blueprints/BP_ThirdPersonCharacter.HandGrab` (`self.Owner`))))
  ;[0.002064 1 0.1104 1 50] WorkingCable
  (if (`self.GrapOnCd`)
    _
    (elif (not (`self.bHasUsedGrap`))
      (set `self.bHasUsedGrap` true)
      (`self.CE_GrapTiming`)
      (bind (_outhit _returnvalue_2) (`KismetSystemLibrary.LineTraceSingle` :`Start` _returnvalue :`End` (+ (* (`SceneComponent.GetForwardVector` (`/Game/_Core/ThirdPerson/Blueprints/BP_ThirdPersonCharacter.FollowCamera` (`self.Owner`))) 1500.0) _returnvalue) :`TraceChannel` "TraceTypeQuery1" :`DrawDebugType` "Persistent"))
      (if _returnvalue_2
        (bind (_bblockinghit _binitialoverlap _time _distance _location _impactpoint _normal _impactnormal _physmat) (`GameplayStatics.BreakHitResult` _outhit))
        (if (select `EPhysicalSurface` (`PhysicalMaterial.SurfaceType` _physmat) :`SurfaceType1` true)
          (set `self.Impact Point` _impactpoint)
          (`Character.LaunchCharacter` (`self.Owner`) (+ (* (`KismetMathLibrary.Normal` (+ (`KismetMathLibrary.GetDirectionUnitVector` (`Actor.K2_GetActorLocation` (`self.Owner`)) (`self.Impact Point`)) (* (* `WheelMouse input` (`Actor.GetActorRightVector` (`self.Owner`))) 0.5))) (`self.VelocityModifier`)) (0.0 0.0 0.0)) false false)
          (`KismetSystemLibrary.Delay` 0.15)
          (set `self.bGrapplingJump` true)
          (`CharacterMovementComponent.SetMovementMode` (`Character.CharacterMovement` _owner) "MOVE_Flying" 0)
          (bind _returnvalue_3 (`|SpawnActorFromClass` "/Game/_Core/Blueprints/Objects/Grapple/Bp_Rope.Bp_Rope_C" (`KismetMathLibrary.MakeTransform` (`self.Impact Point`)) "Undefined" "MultiplyWithRoot" null (`KismetMathLibrary.Vector_Distance` (`Actor.K2_GetActorLocation` _owner) (`self.Impact Point`)) null))
          (bind _output_get (set `self.Rope` _returnvalue_3))
          (`CableComponent.SetAttachEndTo` (`/Game/_Core/Blueprints/Objects/Grapple/Bp_Rope.Cable` _output_get) (`GameplayStatics.GetPlayerCharacter` 0) "None" "None")
          (`PhysicsConstraintComponent.SetConstrainedComponents` (`/Game/_Core/Blueprints/Objects/Grapple/Bp_Rope.PhysicsConstraint` _output_get) _capsulecomponent "None" null "None")
          (`PrimitiveComponent.SetSimulatePhysics` _capsulecomponent true)
          (`SceneComponent.SetVisibility` (`/Game/_Core/Blueprints/Objects/Grapple/Bp_Rope.Cable` (`self.Rope`)) true false)
          (else
            (`self.CE_CancelHookTrace` :!label _label_2)))
        (else
          (goto _label_2))))))

(event `CE_GrapTiming`
  ;[0.002064 1 0.1104 1 50] WorkingCable
  (set `self.GrapOnCd` true)
  (`KismetSystemLibrary.Delay` (`self.GrapReloadTIming`))
  (set `self.GrapOnCd` false))

(fn `CancelGrappin`
  (bind _owner (`self.Owner`))
  (bind (_returnvalue_roll _returnvalue_pitch _returnvalue_yaw) (`KismetMathLibrary.BreakRotator` (`Pawn.GetControlRotation` _owner)))
  (bind _capsulecomponent (`Character.CapsuleComponent` _owner))
  (`/Engine/EditorBlueprintResources/StandardMacros.IsValid` (`self.Rope`)
    (:`Is Valid`
      (`CharacterMovementComponent.SetMovementMode` (`Character.CharacterMovement` _owner) "MOVE_Falling" 0)
      (`PrimitiveComponent.SetSimulatePhysics` _capsulecomponent false)
      (`SceneComponent.K2_SetWorldRotation` _capsulecomponent (`KismetMathLibrary.MakeRotator` 0.0 0.0 _returnvalue_yaw) false false)
      (`PhysicsConstraintComponent.SetConstrainedComponents` (`/Game/_Core/Blueprints/Objects/Grapple/Bp_Rope.PhysicsConstraint` (`self.Rope`)) null "None" null "None"))))