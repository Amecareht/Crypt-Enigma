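; Health component that tracks its owner's current health, starting at maximum, and handles damage, healing and death.
; Damage and healing clamp health and broadcast value changes, while forced damage bypasses the no-damage and can-take-damage gate.
; At zero health it blocks further changes, broadcasts death with the owner, and asks BP_ThirdPersonGameMode to respawn the player, without checking whether the owner is the player.
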(event `self.ReceiveBeginPlay`
  (set `self.CurrentHealth` (`self.MaxHealth`)))

(event `TakeDamage`
  (params (Damage :type "Float (double-precision)") (ForceDamage :type Boolean))
  ;[0.62 0 0] Damage
  (if (`self.isDead`)
    _
    (elif ForceDamage
      (bind _output_get (set `self.CurrentHealth` (`KismetMathLibrary.FClamp` (- (`self.CurrentHealth`) Damage) 0.0 (`self.MaxHealth`)) :!label _label))
      (`self.HpValueChanged` _output_get (`self.MaxHealth`) true)
      (if (<= _output_get 0.0)
        (`KismetSystemLibrary.PrintString` "Dead")
        (`self.OnDeath_Event`)
        (else
          (`KismetSystemLibrary.PrintString` "TookDamage")))
      (elif (`self.HaveNoDamage`)
        (if (`self.CanTakeDamage`)
          (goto _label))
        (else
          (goto _label))))))

(event `Heal`
  (params (Heal :type "Float (double-precision)"))
  ;[0.04315 0.63 0] Heal
  (if (not (`self.isDead`))
    (bind _output_get (set `self.CurrentHealth` (`KismetMathLibrary.FClamp` (+ (`self.CurrentHealth`) Heal) 0.0 (`self.MaxHealth`))))
    (`self.HpValueChanged` _output_get (`self.MaxHealth`))))

(event `OnDeath_Event`
  (set `self.isDead` true)
  (`self.OnDeath` (`self.GetOwner`))
  (bind _asbp_third_person_game_mode (cast `/Game/_Core/ThirdPerson/Blueprints/BP_ThirdPersonGameMode` (`GameplayStatics.GetGameMode`)))
  (`/Game/_Core/ThirdPerson/Blueprints/BP_ThirdPersonGameMode.Respawn Player` _asbp_third_person_game_mode))