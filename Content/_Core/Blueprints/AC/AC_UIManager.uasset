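; Actor component that creates and updates health bar widgets and the circle-order UI.
; After a startup delay, it picks the Bossy, player or Anubis bar by owner class or interface; the Anubis bar is never added to the viewport here.
; AC_Health change events drive each bar and unbind at zero health.
; ResetOrderUI flip-flops the initially hidden order widget, toggling cursor and input mode.
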(event `WidgetHp_AnubisChange`
  (params (CurrentHealth :type "Float (double-precision)") (MaxHealth :type "Float (double-precision)") (Damage :type Boolean))
  ;[0.42 0 0] Ui Updater setup Anubis
  (if (== CurrentHealth 0.0)
    (`/Game/_Core/IA/Health/WBP_AnubisHealthBar.UpdateHealth` (`self.AnubisHealthBar`) CurrentHealth MaxHealth)
    (clear `/Game/_Core/Blueprints/AC/AC_Health.HpValueChanged` (`Actor.GetComponentByClass` (`self.GetOwner`) "/Game/_Core/Blueprints/AC/AC_Health.AC_Health_C"))
    (else
      (`/Game/_Core/IA/Health/WBP_AnubisHealthBar.UpdateHealth` (`self.AnubisHealthBar`) CurrentHealth MaxHealth))))

(event `self.ReceiveBeginPlay`
  (bind _returnvalue (`KismetSystemLibrary.DoesImplementInterface` (`self.GetOwner`) "/Game/_Core/Blueprints/BPI/BPI_ReturnPlayer.BPI_ReturnPlayer_C"))
  ;[0.9154 1 0.05] UI Setup
  (`|ExecutionSequence`
    (:`then_0`
      (bind _returnvalue_2 (`|CreateWidget` "/Game/_Core/Blueprints/Widget/MigratedUI/Blueprints/WDJ_CircleOrder.WDJ_CircleOrder_C" (`GameplayStatics.GetPlayerController` 0)))
      (bind _output_get (set `self.WDJ_Test` _returnvalue_2))
      (`UserWidget.AddToViewport` _output_get 0)
      (`Widget.SetVisibility` (`self.WDJ_Test`) "Hidden"))
    (:`then_1`
      (`KismetSystemLibrary.Delay` 4.5)
      (if (== (`GameplayStatics.GetObjectClass` (`self.GetOwner`)) "/Game/_Core/IA/Boss_Sphere/Bossy_Sphere.Bossy_Sphere_C")
        (bind _returnvalue_3 (`|CreateWidget` "/Game/_Core/IA/Health/WBP_bossyHealthBar1.WBP_bossyHealthBar1_C"))
        (bind _output_get_2 (set `self.Bossy_HealthBar` _returnvalue_3))
        (`UserWidget.AddToViewport` _output_get_2 0)
        ;[0.42 0 0] Ui Updater setup Player
        (add `/Game/_Core/Blueprints/AC/AC_Health.HpValueChanged` (`Actor.GetComponentByClass` (`self.GetOwner`) "/Game/_Core/Blueprints/AC/AC_Health.AC_Health_C") (delegate `Widget_Bossy_Change`))
        (else
          (if _returnvalue
            (bind _returnvalue_4 (`|CreateWidget` "/Game/_Core/Blueprints/Widget/WBP_HealthBar.WBP_HealthBar_C"))
            (bind _output_get_3 (set `self.HealthBar` _returnvalue_4))
            (`UserWidget.AddToViewport` _output_get_3 0)
            (else
              (bind _returnvalue_5 (`|CreateWidget` "/Game/_Core/IA/Health/WBP_AnubisHealthBar.WBP_AnubisHealthBar_C"))
              (set `self.AnubisHealthBar` _returnvalue_5)))
          (if _returnvalue
            ;[0.42 0 0] Ui Updater setup Player
            (add `/Game/_Core/Blueprints/AC/AC_Health.HpValueChanged` (`Actor.GetComponentByClass` (`GameplayStatics.GetPlayerPawn` 0) "/Game/_Core/Blueprints/AC/AC_Health.AC_Health_C") (delegate `WidgetHpChange`))
            (else
              ;[0.42 0 0] Ui Updater setup Anubis
              (add `/Game/_Core/Blueprints/AC/AC_Health.HpValueChanged` (`Actor.GetComponentByClass` (`self.GetOwner`) "/Game/_Core/Blueprints/AC/AC_Health.AC_Health_C") (delegate `WidgetHp_AnubisChange`)))))))))

(event `WidgetHpChange`
  (params (CurrentHealth :type "Float (double-precision)") (MaxHealth :type "Float (double-precision)") (Damage :type Boolean))
  ;[0.42 0 0] Ui Updater setup Player
  (if (== CurrentHealth 0.0)
    (`/Game/_Core/Blueprints/Widget/WBP_HealthBar.UpdateHealth` (`self.HealthBar`) CurrentHealth MaxHealth)
    (clear `/Game/_Core/Blueprints/AC/AC_Health.HpValueChanged` (`Actor.GetComponentByClass` (`GameplayStatics.GetPlayerPawn` 0) "/Game/_Core/Blueprints/AC/AC_Health.AC_Health_C"))
    (else
      (`/Game/_Core/Blueprints/Widget/WBP_HealthBar.UpdateHealth` (`self.HealthBar`) CurrentHealth MaxHealth))))

(event `StartUIOrder`)

(event `ResetOrderUI`
  (bind _wdj_test (`self.WDJ_Test`))
  (bind _isa (`/Engine/EditorBlueprintResources/StandardMacros.FlipFlop`)
    (:`A`
      (set `self.Is A` _isa)
      (set `PlayerController.bShowMouseCursor` true (`GameplayStatics.GetPlayerController` 0))
      (`Widget.SetVisibility` _wdj_test "Visible")
      (`WidgetBlueprintLibrary.SetInputMode_GameAndUIEx` (`GameplayStatics.GetPlayerController` 0) _wdj_test "DoNotLock" false))
    (:`B`
      (set `self.Is A` _isa)
      (set `PlayerController.bShowMouseCursor` false (`GameplayStatics.GetPlayerController` 0))
      (`Widget.SetVisibility` (`self.WDJ_Test`) "Hidden")
      (`WidgetBlueprintLibrary.SetInputMode_GameOnly` (`GameplayStatics.GetPlayerController` 0)))))

(event `Widget_Bossy_Change`
  (params (CurrentHealth :type "Float (double-precision)") (MaxHealth :type "Float (double-precision)") (Damage :type Boolean))
  ;[0.42 0 0] Ui Updater setup Player
  (if (== CurrentHealth 0.0)
    (`/Game/_Core/IA/Health/WBP_bossyHealthBar1.UpdateHealth` (`self.Bossy_HealthBar`) CurrentHealth MaxHealth)
    (clear `/Game/_Core/Blueprints/AC/AC_Health.HpValueChanged` (`Actor.GetComponentByClass` (`self.GetOwner`) "/Game/_Core/Blueprints/AC/AC_Health.AC_Health_C"))
    (else
      (`/Game/_Core/IA/Health/WBP_bossyHealthBar1.UpdateHealth` (`self.Bossy_HealthBar`) CurrentHealth MaxHealth))))