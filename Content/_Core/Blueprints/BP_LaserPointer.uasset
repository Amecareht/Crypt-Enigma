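; BP_LaserPointer is a laser pointer visual that displays a Niagara beam.
; The beam is hidden on BeginPlay, and the StartLaserVisual and EndLaserVisual events show and hide it.
; OnGoingLaser receives an end location and writes it to the Niagara "Beam End" vector parameter.
; The Blueprint does no tracing or input handling itself, only exposing these events to drive the effect.
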(event `self.ReceiveBeginPlay`
  (`SceneComponent.SetVisibility` (`self.Niagara`) false false))

(event `StartLaserVisual`
  (`SceneComponent.SetVisibility` (`self.Niagara`) true false))

(event `EndLaserVisual`
  (`SceneComponent.SetVisibility` (`self.Niagara`) false false))

(event `OnGoingLaser`
  (params (EndLocation :type "Vector Structure"))
  (`FXSystemComponent.SetVectorParameter` (`self.Niagara`) "Beam End" EndLocation))

(fn `UserConstructionScript`)