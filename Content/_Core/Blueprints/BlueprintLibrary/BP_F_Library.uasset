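; BP_F_Library is a Blueprint function library with one helper, SlerpWithSegment, apparently meant for arc-style interpolation between two points.
; It scales the XY heading from Start to End by Alpha and builds a flat direction vector from that angle.
; That vector multiplies the sum of the segment midpoint and full Start-to-End distance, rather than being offset from the midpoint.
; The LerpedValue input does not affect the result.
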(fn `SlerpWithSegment`
  (params (Start :type "Vector Structure") (End :type "Vector Structure") (LerpedValue :type "Vector Structure") (Alpha :type "Float (double-precision)" :default 180.0))
  (returns (SlerpPos :type "Vector Structure"))
  (locals (Centre :type "Vector Structure") (Radius :type "Float (double-precision)") (Angle :type "Float (double-precision)") (AngleTotal :type "Float (double-precision)") (X :type "Float (double-precision)") (Y :type "Float (double-precision)") (Z :type "Float (double-precision)"))
  (bind (_returnvalue_x _returnvalue_y) (`KismetMathLibrary.BreakVector` (- End Start)))
  (bind _returnvalue (`KismetMathLibrary.RadiansToDegrees` (`KismetMathLibrary.Atan2` _returnvalue_y _returnvalue_x)))
  (set `local.Centre` (/ (+ Start End) 2))
  (set `local.Radius` (`KismetMathLibrary.Vector_Distance` (`local.Start`) (`local.End`)))
  (set `local.AngleTotal` _returnvalue)
  (set `local.Angle` (* _returnvalue (`local.Alpha`)))
  (set `local.X` 0.0)
  (return (* (+ (`local.Radius`) (`local.Centre`)) (`KismetMathLibrary.MakeVector` (`KismetMathLibrary.Cos` (`KismetMathLibrary.DegreesToRadians` (`local.Angle`))) (`KismetMathLibrary.Sin` (`KismetMathLibrary.DegreesToRadians` (`local.Angle`)))))))