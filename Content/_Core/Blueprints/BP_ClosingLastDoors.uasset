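; Trigger volume that closes the last doors behind the player and wakes the Bossy_Sphere boss.
; When the player character overlaps its box, it calls BossyWakeUp on the Bossy_Sphere actor found in the level.
; It then finds the first actors tagged LeftDoor and RightDoor and snaps each instantly to its stored absolute end location, with no sweep or animation.
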(event `self.Box.OnComponentBeginOverlap`
  (params (OverlappedComponent :type "PrimitiveComponent Object Reference") (OtherActor :type "Actor Object Reference") (OtherComp :type "PrimitiveComponent Object Reference") (OtherBodyIndex :type Integer) (bFromSweep :type Boolean) (SweepResult :type "HitResult Structure (by ref)"))
  (if (== OtherActor (`GameplayStatics.GetPlayerCharacter` 0))
    (bind _returnvalue (`GameplayStatics.GetActorOfClass` "/Game/_Core/IA/Boss_Sphere/Bossy_Sphere.Bossy_Sphere_C"))
    (`/Game/_Core/IA/Boss_Sphere/Bossy_Sphere.Bossy_WakeUp` _returnvalue)
    (`|ExecutionSequence`
      (:`then_0`
        (bind _outactors (`GameplayStatics.GetAllActorsWithTag` "LeftDoor"))
        (`self.K2_SetActorLocation` (`|GetArrayItem` _outactors) (`self.EndLocLeftDoor`) false false))
      (:`then_1`
        (bind _outactors_2 (`GameplayStatics.GetAllActorsWithTag` "RightDoor"))
        (`self.K2_SetActorLocation` (`|GetArrayItem` _outactors_2) (`self.EndLocRightDoor`) false false)))))

(fn `UserConstructionScript`)