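; PC_Rider is the rider's player controller, which owns the radial command HUD used to give orders to the horse.
; On BeginPlay it creates the hidden WDJ_CircleOrder widget, then, if the player character is a BP_Rider, caches it, initializes the widget and loads game user settings.
; ResetOrderUI either shows the widget with Game and UI input or, on forced deactivation, hides it and restores game-only input.
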(event `self.ReceiveBeginPlay`
  (bind _returnvalue (`GameplayStatics.GetPlayerCharacter` 0))
  (bind _returnvalue_2 (`|CreateWidget` "/Game/_Core/Blueprints/Widget/MigratedUI/Blueprints/WDJ_CircleOrder.WDJ_CircleOrder_C" self))
  (bind _output_get (set `self.HUDCircleCommand` _returnvalue_2))
  (`UserWidget.AddToViewport` _output_get 0)
  (`Widget.SetVisibility` (`self.HUDCircleCommand`) "Hidden")
  (`/Engine/EditorBlueprintResources/StandardMacros.IsValid` _returnvalue
    (:`Is Valid`
      (bind _asbp_rider (cast `/Game/UltimateHorsePack/Blueprints/BP_Rider` _returnvalue))
      (set `self.BP_Rider` _asbp_rider)
      (`/Game/_Core/Blueprints/Widget/MigratedUI/Blueprints/WDJ_CircleOrder.OninitializedPC_Rider` (`self.HUDCircleCommand`))
      (bind _returnvalue_3 (`GameUserSettings.GetGameUserSettings`))
      (`GameUserSettings.LoadSettings` _returnvalue_3 false))))

(event `ResetOrderUI`
  (params (ForceDesactivation :type Boolean))
  (bind _returnvalue (`GameplayStatics.GetPlayerController` 0))
  ;[1 1 1] HUD CommandHorse start/end
  (if ForceDesactivation
    (`Widget.SetVisibility` (`self.HUDCircleCommand`) "Hidden")
    (`WidgetBlueprintLibrary.SetInputMode_GameOnly` _returnvalue)
    (else
      (`Widget.SetVisibility` (`self.HUDCircleCommand`) "Visible")
      (`WidgetBlueprintLibrary.SetInputMode_GameAndUIEx` _returnvalue null))))

(fn `UserConstructionScript`)