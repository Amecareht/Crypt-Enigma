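; Destructible block for the sphere boss that launches itself at the player's BP_Rider.
; On BeginPlay it binds a rotating movement to its geometry collection, then after a short delay glides its root to the rider's location with a timed MoveComponentTo.
; Tick caches the rider and turns the root to face it.
; Hit only prints debug text, and the logic to enable gravity and stop the spin is unconnected.
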(event `self.ReceiveBeginPlay`
  (`MovementComponent.SetUpdatedComponent` (`self.RotatingMovement`) (`self.Destroyed_Block_GeometryCollection`))
  (`KismetSystemLibrary.Delay` 2.0)
  (`KismetSystemLibrary.PrintString` "Test delay")
  (`KismetSystemLibrary.MoveComponentTo` (`self.Root`) (`self.K2_GetActorLocation` (stale `self.ReceiveTick` _asbp_rider)) (struct) false false 3.0))

(event `self.ReceiveTick`
  (params (DeltaSeconds :type "Float (single-precision)"))
  (bind _asbp_rider (cast `/Game/UltimateHorsePack/Blueprints/BP_Rider` (`GameplayStatics.GetPlayerPawn` 0)))
  (`SceneComponent.K2_SetWorldRotation` (`self.Root`) (`KismetMathLibrary.FindLookAtRotation` (`self.K2_GetActorLocation`) (`self.K2_GetActorLocation` _asbp_rider)) true false))

(event `self.ReceiveHit`
  (params (MyComp :type "PrimitiveComponent Object Reference") (Other :type "Actor Object Reference") (OtherComp :type "PrimitiveComponent Object Reference") (bSelfMoved :type Boolean) (HitLocation :type "Vector Structure") (HitNormal :type "Vector Structure") (NormalImpulse :type "Vector Structure") (Hit :type "HitResult Structure (by ref)"))
  (set `self.Touched_Surface` (`GameplayStatics.BreakHitResult` Hit))
  (if (`self.Touched_Surface`)
    (`KismetSystemLibrary.PrintString` "hit")))

(fn `UserConstructionScript`)