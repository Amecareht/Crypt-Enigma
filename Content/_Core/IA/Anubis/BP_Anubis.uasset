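; Anubis boss character that sits until Bossy_Sphere reaches its last position, then wakes up and chases the player.
; It loops AI move-to into stomp montages; once the stomp count runs out, it enters a flying phase that spawns an attached cube projectile, then resets.
; Timelines drive turning toward the player, and damage routes to a health component, with a heal damage type restoring health.
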(event `self.ReceiveTick`
  (params (DeltaSeconds :type "Float (single-precision)"))
  (`|ExecutionSequence`
    (:`then_0`
      (`self.Check if it can start`))))

(event `self.ReceiveAnyDamage`
  (params (Damage :type "Float (single-precision)") (DamageType :type "DamageType Object Reference") (InstigatedBy :type "Controller Object Reference") (DamageCauser :type "Actor Object Reference"))
  (bind _ac_health (`self.AC_Health`))
  ;[1 1 1] Life Anubis
  (if (== (`GameplayStatics.GetObjectClass` DamageType) "/Game/_Core/Blueprints/FrameWorks/DamageType_Heal.DamageType_Heal_C")
    (`/Game/_Core/Blueprints/AC/AC_Health.Heal` _ac_health Damage)
    (else
      (`/Game/_Core/Blueprints/AC/AC_Health.TakeDamage` _ac_health Damage false))))

(event `self.ReceiveBeginPlay`
  ;[1 1 1] Start to check
  (set `self.Stomp Count` 3)
  (set `/Game/_Core/Blueprints/AC/AC_Health.CurrentHealth` 100.0 (`self.AC_Health`))
  (add `/Game/_Core/Blueprints/AC/AC_Health.OnDeath` (`self.AC_Health`) (`|CreateDelegate` :!event `Die`)))

(event `Move to`
  (params (WakingUp :type Boolean))
  ;[1 1 1] Check if it can start to getting up
  (set `self.Back to idlle` true)
  (`KismetSystemLibrary.PrintString` "Move to target")
  (`|AIMoveTo` self (0.0 0.0 0.0) (`GameplayStatics.GetPlayerCharacter` 0) 1500.0
    (:`OnSuccess`
      (`KismetSystemLibrary.PrintString` "move to successful")
      (`self.Attack Player`))))

(event `Check if it can start`
  ;[1 1 1] Check if it can start to getting up
  (bind _returnvalue (`GameplayStatics.GetActorOfClass` "/Game/_Core/IA/Boss_Sphere/Bossy_Sphere.Bossy_Sphere_C"))
  (if (`/Game/_Core/IA/Boss_Sphere/Bossy_Sphere.Is in the last pos` _returnvalue)
    (`/Engine/EditorBlueprintResources/StandardMacros.DoOnce` false
      (:`Completed`
        (set `self.Sit` false)
        (set `self.WakingUp` true)
        (`KismetSystemLibrary.PrintString` "waking up")
        (`ActorComponent.Activate` (`self.Anubis_Vocals_V4__loop__Cue`) false)
        (`KismetSystemLibrary.Delay` 11.0)
        (set `self.WakingUp` (stale `Move to` WakingUp))
        (set `self.Ready To fight` true)
        (`KismetSystemLibrary.PrintString` "Anubis Ready to fight")
        (`self.Move to` false)))
    (else
      (set `self.Sit` true))))

(event `Attack Player`
  (bind _arrow1 (`self.Arrow1`))
  (bind (_returnvalue_roll _returnvalue_pitch _returnvalue_yaw) (`KismetMathLibrary.BreakRotator` (`KismetMathLibrary.FindLookAtRotation` (`self.K2_GetActorLocation`) (`self.K2_GetActorLocation` (`GameplayStatics.GetPlayerCharacter` 0)))))
  ;[1 1 1] Attack
  (`SceneComponent.K2_SetWorldRotation` (`self.CapsuleComponent`) (`KismetMathLibrary.MakeRotator` 0.0 0.0 _returnvalue_yaw) false false)
  (if (> (`self.Stomp Count`) 0)
    (`|PlayMontage` (`self.Mesh`) "/Game/_Core/IA/Anubis/Animation/Anubis_Stomp_Montage.Anubis_Stomp_Montage"
      (:`OnCompleted`
        (`KismetSystemLibrary.Delay` 1.0)
        (set `self.Stomp Count` (- (`self.Stomp Count`) 1))
        (`self.Move to` false)))
    (else
      (bind _returnvalue (`GameplayStatics.GetActorOfClass` "/Game/_Core/IA/Boss_Sphere/Anubis_ThrowPoint.Anubis_ThrowPoint_C"))
      (set `self.StartFlying` true)
      (`KismetSystemLibrary.K2_SetTimerDelegate` (delegate `Face plyer`) 0.01 true)
      (bind (_direction _scale) (`Timeline|Timeline_0` :!via `PlayFromStart`)
        (:`Update`
          (set `self.Final location` (`KismetMathLibrary.VLerp` (`self.K2_GetActorLocation`) (`SceneComponent.K2_GetComponentLocation` (`/Game/_Core/IA/Boss_Sphere/Anubis_ThrowPoint.DefaultSceneRoot` _returnvalue)) _scale))
          (set `self.Fly` true)
          (`KismetSystemLibrary.Delay` 3.0)
          (`GameplayStatics.SpawnEmitterAttached` "/Game/_Core/IA/Boss_Sphere/FXVarietyPack/Particles/Spawner_FX.Spawner_FX" _arrow1 "None" (`SceneComponent.K2_GetComponentLocation` _arrow1) (struct) (1.0 1.0 1.0) "SnapToTarget")
          (bind _returnvalue_2 (`|SpawnActorFromClass` "/Game/_Core/IA/Boss_Sphere/Cube_Projectile.Cube_Projectile_C" (`KismetMathLibrary.Conv_VectorToTransform` (`SceneComponent.K2_GetComponentLocation` _arrow1)) "AlwaysSpawn" "MultiplyWithRoot" null null))
          (`self.K2_AttachToComponent` _returnvalue_2 _arrow1 "None" "KeepWorld" "KeepWorld" "KeepWorld" true)
          (`KismetSystemLibrary.Delay` 10.0)
          (set `self.Fly` false)
          (set `self.StartFlying` false)
          (set `self.EndFlying` true)
          (set `self.Stomp Count` 3)
          (`self.Move to` false))))))

(event `self.PawnSensing.OnSeePawn`
  (params (Pawn :type "Pawn Object Reference"))
  ;[1 1 1] Check if it can Follow
)

(event `Follow player`
  ;[1 1 1] Follow
  (if (`self.IsSeeingPlayer`)
    _))

(event `Face plyer`
  (bind (_returnvalue_roll _returnvalue_pitch _returnvalue_yaw) (`KismetMathLibrary.BreakRotator` (`SceneComponent.K2_GetComponentRotation` (`self.CapsuleComponent`))))
  (bind (_returnvalue_roll_2 _returnvalue_pitch_2 _returnvalue_yaw_2) (`KismetMathLibrary.BreakRotator` (`KismetMathLibrary.FindLookAtRotation` (`self.K2_GetActorLocation`) (`self.K2_GetActorLocation` (`GameplayStatics.GetPlayerCharacter` 0)))))
  ;[1 1 1] Attack
  (bind (_direction _scale) (`Timeline|Timeline` :!via `PlayFromStart`)
    (:`Update`
      (bind _output_get (set `self.Final rotation` (`KismetMathLibrary.MakeRotator` 0.0 0.0 (`KismetMathLibrary.Lerp` _returnvalue_yaw _returnvalue_yaw_2 _scale))))
      (`SceneComponent.K2_SetWorldRotation` (`self.CapsuleComponent`) (`KismetMathLibrary.MakeRotator` 0.0 0.0 (.yaw _output_get)) false false))))

(event `Die`
  (params (RefToSelf :type "Actor Object Reference"))
  (clear `/Game/_Core/Blueprints/AC/AC_Health.OnDeath` (`self.AC_Health`))
  (`|PlayMontage` (`self.Mesh`) "/Game/_Core/IA/Anubis/Animation/Anubis_Death_Montage.Anubis_Death_Montage"))

(fn `UserConstructionScript`)