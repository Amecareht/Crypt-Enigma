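; BP_FakeSkeleton is a fake skeleton that travels along a designer-placed spline using InterpToMovement.
; On BeginPlay it copies the spline points into relative control points, sets the duration from DurationEnd and sets the initial tick state from Active.
; A toggle event switches movement by component tick, honoring the requested state only when NeedToStayOff is set and otherwise keeping it ticking.
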(event `self.ReceiveBeginPlay`
  (`self.SetControlPoint`)
  (`self.Initial` (`self.Active`))
  (`self.Toogle_Movement` true))

(event `SetControlPoint`
  (bind _interptomovement (`self.InterpToMovement`))
  (for _index (range (`SplineComponent.GetNumberOfSplinePoints` (`self.Spline`)))
    (`InterpToMovementComponent.AddControlPointPosition` (`self.InterpToMovement`) (`SplineComponent.GetLocationAtSplinePoint` (`self.Spline`) _index "Local") true))
  (set `InterpToMovementComponent.Duration` (`self.DurationEnd`) _interptomovement)
  (`InterpToMovementComponent.FinaliseControlPoints` _interptomovement))

(event `Toogle_Movement`
  (params (Enable :type Boolean))
  (bind _interptomovement (`self.InterpToMovement`))
  (if (`self.NeedToStayOff`)
    (`ActorComponent.SetComponentTickEnabled` _interptomovement Enable)
    (else
      (`ActorComponent.SetComponentTickEnabled` _interptomovement true))))

(event `Initial`
  (params (Enable :type Boolean))
  (bind _interptomovement (`self.InterpToMovement`))
  (`ActorComponent.SetComponentTickEnabled` _interptomovement Enable)
  (`ActorComponent.Activate` _interptomovement false))

(fn `UserConstructionScript`)