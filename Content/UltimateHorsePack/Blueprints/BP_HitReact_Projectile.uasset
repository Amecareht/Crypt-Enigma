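; BP_HitReact_Projectile is a physics cube projectile that triggers hit reactions on BP_Horse actors it strikes.
; On BeginPlay it launches along its forward vector with a velocity-change impulse.
; After a short delay, a Despawn timeline drives the cube's scale, then destroys the actor.
; A component hit on a horse passes the impact location to its HitReact, limited to once per projectile by a DoOnce.
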(event `self.ReceiveBeginPlay`
  (`PrimitiveComponent.AddImpulse` (`self.Cube`) (* (`SceneComponent.GetForwardVector` (`self.Cube`)) 2000.0) "None" true)
  (`KismetSystemLibrary.Delay` 2.0)
  (bind (_direction _scale) (`Timeline|Despawn` :!via `PlayFromStart`)
    (:`Update`
      (`SceneComponent.SetWorldScale3D` (`self.Cube`) (`KismetMathLibrary.Conv_DoubleToVector` _scale)))
    (:`Finished`
      (`self.K2_DestroyActor`))))

(event `self.Cube.OnComponentHit`
  (params (HitComponent :type "PrimitiveComponent Object Reference") (OtherActor :type "Actor Object Reference") (OtherComp :type "PrimitiveComponent Object Reference") (NormalImpulse :type "Vector Structure") (Hit :type "HitResult Structure (by ref)"))
  (bind _asbp_horse (cast `/Game/UltimateHorsePack/Blueprints/BP_Horse` OtherActor))
  (`/Engine/EditorBlueprintResources/StandardMacros.DoOnce` false
    (:`Completed`
      (`/Game/UltimateHorsePack/Blueprints/BP_Horse.Hit React` _asbp_horse (`.Location` (`GameplayStatics.BreakHitResult` Hit))))))

(fn `UserConstructionScript`)