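; Preview saddle actor from the horse pack, with a skeletal saddle mesh, bags and a hat.
; SetupBodies turns on physics below the bag, rope, flask and hat socket bones.
; UpdateTexture picks one of five material presets and passes it to SetupMaterials, which applies it to saddle slots, bags and hat.
; SocketHattoHand reattaches the hat to a given character's hand socket.
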(event `Setup Bodies`
  (`SkeletalMeshComponent.SetAllBodiesBelowSimulatePhysics` (`self.Saddle_mesh`) "Socket_left_Bag" true true)
  (`SkeletalMeshComponent.SetAllBodiesBelowSimulatePhysics` (`self.Saddle_mesh`) "Socket_left_SideBag" true true)
  (`SkeletalMeshComponent.SetAllBodiesBelowSimulatePhysics` (`self.Saddle_mesh`) "Socket_right_Sidebag" true true)
  (`SkeletalMeshComponent.SetAllBodiesBelowSimulatePhysics` (`self.Saddle_mesh`) "Socket_right_bag" true true)
  (`SkeletalMeshComponent.SetAllBodiesBelowSimulatePhysics` (`self.Saddle_mesh`) "Socket_Rope" true true)
  (`SkeletalMeshComponent.SetAllBodiesBelowSimulatePhysics` (`self.Saddle_mesh`) "Socket_Flask" true true)
  (`SkeletalMeshComponent.SetAllBodiesBelowSimulatePhysics` (`self.Saddle_mesh`) "Socket_Hat" true true))

(event `Socket Hat to Hand`
  (params (Character :type "Character Object Reference"))
  (`SceneComponent.K2_AttachToComponent` (`self.hat`) (`Character.Mesh` Character) "rHand_HatSocket" "SnapToTarget" "SnapToTarget" "KeepRelative" true))

(event `self.ReceiveBeginPlay`)

(event `Update Texture`
  (params (Selection :type "/Game/UltimateHorsePack/Blueprints/Enum_AdvancedSaddleVariant Enum" :default "NewEnumerator0"))
  (switch `/Game/UltimateHorsePack/Blueprints/Enum_AdvancedSaddleVariant` Selection
    (:`NewEnumerator0`
      (`self.SetupMaterials` "/Game/UltimateHorsePack/Materials/Saddle/MI_Bridle.MI_Bridle" "/Game/UltimateHorsePack/Materials/Saddle/MI_SaddleSeat2.MI_SaddleSeat2" "/Game/UltimateHorsePack/Materials/Saddle/MI_BeltBits.MI_BeltBits" "/Game/UltimateHorsePack/Materials/Saddle/MI_BeltBack.MI_BeltBack" "/Game/UltimateHorsePack/Materials/Saddle/MI_RectBagTop.MI_RectBagTop" "/Game/UltimateHorsePack/Materials/Saddle/MI_Bag01.MI_Bag01" "/Game/UltimateHorsePack/Materials/Saddle/MI_BagRound01.MI_BagRound01" "/Game/UltimateHorsePack/Materials/Saddle/MI_Hat01.MI_Hat01"))
    (:`NewEnumerator1`
      (`self.SetupMaterials` "/Game/UltimateHorsePack/Materials/Saddle/MI_Bridle2.MI_Bridle2" "/Game/UltimateHorsePack/Materials/Saddle/MI_SaddleSeat5.MI_SaddleSeat5" "/Game/UltimateHorsePack/Materials/Saddle/MI_BeltBits2.MI_BeltBits2" "/Game/UltimateHorsePack/Materials/Saddle/MI_BeltBack.MI_BeltBack" "/Game/UltimateHorsePack/Materials/Saddle/MI_RectBagTop2.MI_RectBagTop2" "/Game/UltimateHorsePack/Materials/Saddle/MI_Bag02.MI_Bag02" "/Game/UltimateHorsePack/Materials/Saddle/MI_BagRound2.MI_BagRound2" "/Game/UltimateHorsePack/Materials/Saddle/MI_Hat03.MI_Hat03"))
    (:`NewEnumerator2`
      (`self.SetupMaterials` "/Game/UltimateHorsePack/Materials/Saddle/MI_Bridle.MI_Bridle" "/Game/UltimateHorsePack/Materials/Saddle/MI_SaddleSeat7.MI_SaddleSeat7" "/Game/UltimateHorsePack/Materials/Saddle/MI_BeltBits.MI_BeltBits" "/Game/UltimateHorsePack/Materials/Saddle/MI_BeltBack.MI_BeltBack" "/Game/UltimateHorsePack/Materials/Saddle/MI_RectBagTop6.MI_RectBagTop6" "/Game/UltimateHorsePack/Materials/Saddle/MI_Bag06.MI_Bag06" "/Game/UltimateHorsePack/Materials/Saddle/MI_BagRound7.MI_BagRound7" "/Game/UltimateHorsePack/Materials/Saddle/MI_Hat04.MI_Hat04"))
    (:`NewEnumerator3`
      (`self.SetupMaterials` "/Game/UltimateHorsePack/Materials/Saddle/MI_Bridle2.MI_Bridle2" "/Game/UltimateHorsePack/Materials/Saddle/PickYourOwnColours/MI_Saddle02_01.MI_Saddle02_01" "/Game/UltimateHorsePack/Materials/Saddle/MI_BeltBits.MI_BeltBits" "/Game/UltimateHorsePack/Materials/Saddle/MI_BeltBack.MI_BeltBack" "/Game/UltimateHorsePack/Materials/Saddle/MI_RectBagTop3.MI_RectBagTop3" "/Game/UltimateHorsePack/Materials/Saddle/MI_Bag03.MI_Bag03" "/Game/UltimateHorsePack/Materials/Saddle/MI_BagRound3.MI_BagRound3" "/Game/UltimateHorsePack/Materials/Saddle/MI_Hat03.MI_Hat03"))
    (:`NewEnumerator4`
      (`self.SetupMaterials` "/Game/UltimateHorsePack/Materials/Saddle/MI_Bridle.MI_Bridle" "/Game/UltimateHorsePack/Materials/Saddle/MI_SaddleSeat5.MI_SaddleSeat5" "/Game/UltimateHorsePack/Materials/Saddle/MI_BeltBits2.MI_BeltBits2" "/Game/UltimateHorsePack/Materials/Saddle/MI_BeltBack.MI_BeltBack" "/Game/UltimateHorsePack/Materials/Saddle/MI_RectBagTop5.MI_RectBagTop5" "/Game/UltimateHorsePack/Materials/Saddle/MI_Bag05.MI_Bag05" "/Game/UltimateHorsePack/Materials/Saddle/MI_BagRound5.MI_BagRound5" "/Game/UltimateHorsePack/Materials/Saddle/MI_Hat02.MI_Hat02"))))

(fn `SetupMaterials`
  (params (Bridle :type "MaterialInterface Object Reference") (SaddleSeat :type "MaterialInterface Object Reference") (BeltBits :type "MaterialInterface Object Reference") (BeltBack :type "MaterialInterface Object Reference") (BackBag :type "MaterialInterface Object Reference") (SideBags :type "MaterialInterface Object Reference") (SideUpperBags :type "MaterialInterface Object Reference") (Hat :type "MaterialInterface Object Reference"))
  (bind _saddle_mesh (`self.Saddle_mesh`))
  (`PrimitiveComponent.SetMaterial` _saddle_mesh 0 Bridle)
  (`PrimitiveComponent.SetMaterial` _saddle_mesh 1 SaddleSeat)
  (`PrimitiveComponent.SetMaterial` _saddle_mesh 2 BeltBits)
  (`PrimitiveComponent.SetMaterial` _saddle_mesh 3 BeltBack)
  (`PrimitiveComponent.SetMaterial` _saddle_mesh 4 BackBag)
  (`PrimitiveComponent.SetMaterial` (`self.RightSideBag`) 0 SideBags)
  (`PrimitiveComponent.SetMaterial` (`self.LeftSideBag`) 0 SideBags)
  (`PrimitiveComponent.SetMaterial` (`self.LeftBag`) 0 SideUpperBags)
  (`PrimitiveComponent.SetMaterial` (`self.RightBag`) 0 SideUpperBags)
  (`PrimitiveComponent.SetMaterial` (`self.hat`) 0 Hat))

(fn `UserConstructionScript`)